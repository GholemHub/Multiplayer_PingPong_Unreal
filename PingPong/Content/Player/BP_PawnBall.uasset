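; Ping-pong ball pawn that bounces around the field and scores when it hits a goal.
; BeginPlay picks a random X direction with fixed positive Y, and Tick feeds that velocity into FloatingPawnMovement.
; Sphere overlaps flip X on BP_Wall or paddle pawns and Y on BP_Wall2, with a collision sound.
; Goal overlaps spawn a replacement ball near the origin, increment the game mode score, play a sound and destroy this ball.
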(event `self.ReceiveBeginPlay`
  (set `self.Velocity` (`KismetMathLibrary.MakeVector` (`KismetMathLibrary.SelectFloat` 1.0 -1.0 (`KismetMathLibrary.RandomBool`)) (`KismetMathLibrary.SelectFloat` 1.0 1.0 (`KismetMathLibrary.RandomBool`)))))

(event `self.ReceiveTick`
  (params (DeltaSeconds :type "Float (single-precision)"))
  (`PawnMovementComponent.AddInputVector` (`self.FloatingPawnMovement`) (`self.Velocity`) false))

(event `self.Sphere1.OnComponentBeginOverlap`
  (params (OverlappedComponent :type "PrimitiveComponent Object Reference") (OtherActor :type "Actor Object Reference") (OtherComp :type "PrimitiveComponent Object Reference") (OtherBodyIndex :type Integer) (bFromSweep :type Boolean) (SweepResult :type "HitResult Structure (by ref)"))
  (bind (_velocity_x _velocity_y _velocity_z) (`KismetMathLibrary.BreakVector` (`self.Velocity`)))
  (bind (_velocity_x_2 _velocity_y_2 _velocity_z_2) (`KismetMathLibrary.BreakVector` (`self.Velocity`)))
  (bind (_velocity_x_3 _velocity_y_3 _velocity_z_3) (`KismetMathLibrary.BreakVector` (`self.Velocity`)))
  (cast `/Game/Player/BP_Wall` OtherActor
    (:`then`
      (set `self.Velocity` (`KismetMathLibrary.MakeVector` (* _velocity_x_2 -1.0) _velocity_y_2 _velocity_z_2))
      (`GameplayStatics.SpawnSound2D` "/Game/Player/Sounds/SCue_Collision.SCue_Collision" 1.0 1.0 0.0 null))
    (:`CastFailed`
      (cast `/Game/Player/BP_BasePawn` OtherActor
        (:`then`
          (set `self.Velocity` (`KismetMathLibrary.MakeVector` (* _velocity_x_3 -1.0) _velocity_y_3 _velocity_z_3))
          (`GameplayStatics.SpawnSound2D` "/Game/Player/Sounds/SCue_Collision.SCue_Collision" 1.0 1.0 0.0 null))
        (:`CastFailed`
          (cast `/Game/BP_Wall2` OtherActor
            (:`then`
              (set `self.Velocity` (`KismetMathLibrary.MakeVector` _velocity_x (* _velocity_y -1.0) _velocity_z))
              (`GameplayStatics.SpawnSound2D` "/Game/Player/Sounds/SCue_Collision.SCue_Collision" 1.0 1.0 0.0 null))
            (:`CastFailed`
              (bind _asbp_goal (cast `/Game/Player/BP_Goal` OtherActor))
              (`self.Goal` (`/Game/Player/BP_Goal.PlayerTargetGoal` _asbp_goal))
              (`GameplayStatics.SpawnSound2D` "/Game/Player/Sounds/SCUE_Goal.SCUE_Goal" 1.0 1.0 0.0 null)
              (`self.K2_DestroyActor`))))))))

(event `Goal`
  (params (PlayerGoal :type Boolean))
  (`|SpawnActorFromClass` "BP_PawnBall_C" (`KismetMathLibrary.MakeTransform` (0.0 0.0 30.0)) "Undefined" "OverrideRootScale" null null)
  (bind _asbp_ping_pong_game_mode_base (cast `/Game/BP_PingPongGameModeBase` (`GameplayStatics.GetGameMode`)))
  (if PlayerGoal
    (bind _result (`/Engine/EditorBlueprintResources/StandardMacros.IncrementInt` (`/Game/BP_PingPongGameModeBase.FirstScore` _asbp_ping_pong_game_mode_base))
      (:`  `
        (set `/Game/BP_PingPongGameModeBase.FirstScore` _result _asbp_ping_pong_game_mode_base)))
    (else
      (bind _result_2 (`/Engine/EditorBlueprintResources/StandardMacros.IncrementInt` (`/Game/BP_PingPongGameModeBase.SecondScore` _asbp_ping_pong_game_mode_base))
        (:`  `
          (set `/Game/BP_PingPongGameModeBase.SecondScore` _result_2 _asbp_ping_pong_game_mode_base)))))
  (`self.K2_DestroyActor`))

(fn `UserConstructionScript`)